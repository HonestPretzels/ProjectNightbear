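; BasicEnemy is a simple test enemy that periodically damages actors around it and can be killed.
; Tick runs through a 1.5-second Delay, throttling attacks that apply AttackDamage to every actor overlapping AttackSphere except itself.
; AnyDamage subtracts truncated damage from Health, which the construction script initializes, then prints a death message and destroys the actor once Health is depleted.
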(event EventBeginPlay)

(event Collision|EventActorBeginOverlap
  (params (OtherActor :type Actor%20Object%20Reference)))

(event EventTick
  (params (DeltaSeconds :type Float%20%28single-precision%29))
  (bind _attack_sphere (Variables|Default|GetAttack%20Sphere))
  (bind _overlappingactors (Collision|GetOverlappingActors _attack_sphere 0 :!class /Script/Engine.PrimitiveComponent))
  (Utilities|FlowControl|Delay 1.5)
  (if (!= (Utilities|Array|LastIndex _overlappingactors) 0)
    (for _array_element _overlappingactors
      (if (not (== _array_element self))
        (Game|Damage|ApplyDamage _array_element (Variables|Default|GetAttack%20Damage) 0 self)))))

(event Game|Damage|EventAnyDamage
  (params (Damage :type Float%20%28single-precision%29) (DamageType :type Damage%20Type%20Object%20Reference) (InstigatedBy :type Controller%20Object%20Reference) (DamageCauser :type Actor%20Object%20Reference))
  (if (Variables|Default|GetAlive)
    (Variables|Default|Sethealth (- (Variables|Default|Gethealth) (Math|Float|Truncate Damage)))
    (if (<= (Variables|Default|Gethealth) 0)
      (Development|PrintString "EnemyDied")
      (Variables|Default|SetAlive false)
      (Actor|DestroyActor))))

(fn ConstructionScript
  (Variables|Default|Sethealth 30))